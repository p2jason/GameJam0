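; BP_Item_Key is a key item actor that shows a pickup widget when a character is near it.
; On BeginPlay it passes itself as the Item to the WBP_ItemPickUp widget in its WidgetComponent.
; SphereCollision overlaps with any Character toggle the widget's visibility on enter and exit.
; The pickup action itself is not handled in this Blueprint's graphs.
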(event `self.ReceiveBeginPlay`
  (bind _aswbp_item_pick_up (cast `/Game/Items/WBP_ItemPickUp` (`WidgetComponent.GetWidget` (`self.WidgetComponent`))))
  (set `/Game/Items/WBP_ItemPickUp.Item` self _aswbp_item_pick_up))

(event `self.SphereCollision.OnComponentBeginOverlap`
  (params (OverlappedComponent :type "PrimitiveComponent Object Reference") (OtherActor :type "Actor Object Reference") (OtherComp :type "PrimitiveComponent Object Reference") (OtherBodyIndex :type Integer) (bFromSweep :type Boolean) (SweepResult :type "HitResult Structure (by ref)"))
  (cast `Character` OtherActor)
  (`SceneComponent.SetVisibility` (`self.WidgetComponent`) true false))

(event `self.SphereCollision.OnComponentEndOverlap`
  (params (OverlappedComponent :type "PrimitiveComponent Object Reference") (OtherActor :type "Actor Object Reference") (OtherComp :type "PrimitiveComponent Object Reference") (OtherBodyIndex :type Integer))
  (cast `Character` OtherActor)
  (`SceneComponent.SetVisibility` (`self.WidgetComponent`) false false))

(fn `UserConstructionScript`)