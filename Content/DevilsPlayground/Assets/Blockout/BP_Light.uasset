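; BP_Light is a proximity-activated light that fades up with a torch sound when an actor begins overlapping it and fades out when an overlap ends.
; Overlap events set a target intensity, and Tick moves the PointLight toward it at TransitionSpeed, clamped between zero and MaxIntensity.
; Starting current intensity below zero forces an initial update to dark.
; An object line trace from the overlapping actor is left unconnected.
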(event `self.ReceiveBeginPlay`
  (set `self.TargetIntensity` 0.0)
  (set `self.CurrentIntensity` -1.0))

(event `self.ReceiveTick`
  (params (DeltaSeconds :type "Float (single-precision)"))
  (if (not (== (`self.TargetIntensity`) (`self.CurrentIntensity`)))
    (if (< (`self.CurrentIntensity`) (`self.TargetIntensity`))
      (set `self.CurrentIntensity` (+ (`self.CurrentIntensity`) (* (`self.TransitionSpeed`) DeltaSeconds)))
      (else
        (bind _output_get (set `self.CurrentIntensity` (+ (`self.CurrentIntensity`) (* DeltaSeconds (* (`self.TransitionSpeed`) -1.0)))))))
    (set `self.CurrentIntensity` (`KismetMathLibrary.FClamp` _output_get 0.0 (`self.MaxIntensity`)))
    (`LightComponent.SetIntensity` (`self.PointLight`) (`self.CurrentIntensity`))))

(event `self.ReceiveActorEndOverlap`
  (params (OtherActor :type "Actor Object Reference"))
  (set `self.TargetIntensity` 0.0))

(event `self.ReceiveActorBeginOverlap`
  (params (OtherActor :type "Actor Object Reference"))
  (set `self.TargetIntensity` (`self.MaxIntensity`))
  (`GameplayStatics.PlaySoundAtLocation` "/Game/DevilsPlayground/Assets/Audio/TorchOnSound.TorchOnSound" (`self.K2_GetActorLocation`) (struct) 1.0 1.0 0.0 null null null null))

(fn `UserConstructionScript`)