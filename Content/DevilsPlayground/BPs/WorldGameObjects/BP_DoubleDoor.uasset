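; Double door actor that swings its two meshes in response to its InteractableComponent's begin and end events.
; Both events set per-door target vectors, with the second target identical in both, but only interaction begin enables Tick.
; Tick calls ApplyRotationToMesh to interpolate each world rotation toward the vector's X-axis rotation at DoorSwingSpeed.
; Tick switches off when both doors, or either one inside that helper, exactly match their target.
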(event `self.ReceiveBeginPlay`
  (bind _interactablecomponent (`self.InteractableComponent`))
  (add `DPInteractableComponent.OnInteractionBegin` _interactablecomponent (delegate `OnInteractionBegin`))
  (add `DPInteractableComponent.OnInteractionEnd` _interactablecomponent (delegate `OnInteractionEnded`)))

(event `OnInteractionBegin`
  (`self.SetActorTickEnabled` true)
  (`KismetMathLibrary.Vector_Set` (`self.TargetRotation`) 0.0 90.0)
  (`KismetMathLibrary.Vector_Set` (`self.TargetRotation2`) 0.0 270.0))

(event `OnInteractionEnded`
  (`KismetMathLibrary.Vector_Set` (`self.TargetRotation`))
  (`KismetMathLibrary.Vector_Set` (`self.TargetRotation2`) 0.0 270.0))

(event `self.ReceiveTick`
  (params (DeltaSeconds :type "Float (single-precision)"))
  (if (and (== (`SceneComponent.K2_GetComponentRotation` (`self.DoorStaticMesh1`)) (`self.TargetRotation`)) (== (`SceneComponent.K2_GetComponentRotation` (`self.DoorStaticMesh2`)) (`self.TargetRotation2`)))
    (`self.SetActorTickEnabled` false)
    (else
      (`self.ApplyRotationToMesh` DeltaSeconds (`self.DoorStaticMesh1`) (`self.TargetRotation`))
      (`self.ApplyRotationToMesh` DeltaSeconds (`self.DoorStaticMesh2`) (`self.TargetRotation2`)))))

(fn `ApplyRotationToMesh`
  (params (FloatSeconds :type "Float (double-precision)") (Mesh :type "StaticMeshComponent Object Reference") (TargetRotation :type "Vector Structure"))
  (bind _returnvalue (`SceneComponent.K2_GetComponentRotation` Mesh))
  (if (== _returnvalue TargetRotation)
    (`self.SetActorTickEnabled` false)
    (else
      (`SceneComponent.K2_SetWorldRotation` Mesh (`KismetMathLibrary.RInterpTo` _returnvalue (`KismetMathLibrary.Conv_VectorToRotator` TargetRotation) FloatSeconds (`self.DoorSwingSpeed`)) false false))))

(fn `UserConstructionScript`)