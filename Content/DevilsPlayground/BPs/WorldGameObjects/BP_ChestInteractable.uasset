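; BP_ChestInteractable is a locked chest the player opens by interacting while holding a key.
; On interaction begin, TryUnlockChest checks the gameplay tag of the item held by the BP_Pleb player character.
; A regular key is removed and destroyed, while a skeleton key is kept.
; Success plays an unlock sound and hides the lid mesh; failure plays a locked sound.
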(event `self.ReceiveBeginPlay`
  (bind _interactablecomponent (`self.InteractableComponent`))
  (add `DPInteractableComponent.OnInteractionBegin` _interactablecomponent (delegate `OnInteractionBegin`))
  (add `DPInteractableComponent.OnInteractionEnd` _interactablecomponent (delegate `OnInteractionEnded`)))

(event `OnInteractionEnded`)

(event `OnInteractionBegin`
  (bind _unlocked (`self.TryUnlockChest`))
  (if _unlocked
    (`GameplayStatics.PlaySound2D` "/Game/DevilsPlayground/Assets/Audio/UnlockSound.UnlockSound" 1.0 1.0 0.0 null null)
    (`SceneComponent.SetHiddenInGame` (`self.ChestLidStaticMesh`) true false)
    (else
      (`GameplayStatics.PlaySound2D` "/Game/DevilsPlayground/Assets/Audio/LockedSound.LockedSound" 1.0 1.0 0.0 null null))))

(fn `TryUnlockChest`
  (returns (Unlocked :type Boolean))
  (bind _asbp_pleb (cast `/Game/DevilsPlayground/BPs/Characters/BP_Pleb` (`GameplayStatics.GetPlayerCharacter` 0)))
  (bind _returnvalue (`DPVillager.GetHeldItem` _asbp_pleb))
  (`/Engine/EditorBlueprintResources/StandardMacros.IsValid` _returnvalue
    (:`Is Valid`
      (`|SwitchGameplayTag` (`ItemBase.ItemTag` _returnvalue)
        (:`Default`
          (return false))
        (:`Items.Key`
          (bind _returnvalue_2 (`DPVillager.RemoveHeldItem` _asbp_pleb))
          (set `self.Is Locked` false)
          (`self.K2_DestroyActor` _returnvalue_2)
          (return true))
        (:`Items.Key.SkeletonKey`
          (set `self.Is Locked` false)
          (return true))))))

(fn `UserConstructionScript`)