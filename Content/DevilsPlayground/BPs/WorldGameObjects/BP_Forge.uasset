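; BP_Forge is an interactable forge that turns the Blacksmith player's held iron into a key.
; On interaction begin from its InteractableComponent, it casts player 0's character to BP_Blacksmith and calls ForgeKey.
; ForgeKey checks the held item for the Iron resource tag, destroys it, then spawns a BP_Item_Key and places it in the Blacksmith's hands.
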(event `self.ReceiveBeginPlay`
  (bind _interactablecomponent (`self.InteractableComponent`))
  (add `DPInteractableComponent.OnInteractionBegin` _interactablecomponent (delegate `OnInteractionBegin`))
  (add `DPInteractableComponent.OnInteractionEnd` _interactablecomponent (delegate `OnInteractionEnded`)))

(event `OnInteractionBegin`
  (bind _asbp_blacksmith (cast `/Game/DevilsPlayground/BPs/Characters/BP_Blacksmith` (`GameplayStatics.GetPlayerCharacter` 0)))
  (`self.ForgeKey` _asbp_blacksmith))

(event `OnInteractionEnded`)

(event `self.ReceiveTick`
  (params (DeltaSeconds :type "Float (single-precision)")))

(fn `ForgeKey`
  (params (Blacksmith :type "/Game/DevilsPlayground/BPs/Characters/BP_Blacksmith Object Reference"))
  (bind _returnvalue (`DPVillager.GetHeldItem` Blacksmith))
  (`/Engine/EditorBlueprintResources/StandardMacros.IsValid` _returnvalue
    (:`Is Valid`
      (if (== (`ItemBase.ItemTag` _returnvalue) (struct :`TagName` "Items.Resources.Iron"))
        (bind _returnvalue_2 (`DPVillager.RemoveHeldItem` Blacksmith))
        (`self.K2_DestroyActor` _returnvalue_2)
        (bind _returnvalue_3 (`|SpawnActorFromClass` "/Game/DevilsPlayground/Items/BP_Item_Key.BP_Item_Key_C" (`KismetMathLibrary.MakeTransform` (0.0 0.0 0.0)) "Undefined" "MultiplyWithRoot" null null))
        (`DPVillager.ReplaceHeldItem` Blacksmith _returnvalue_3)))))

(fn `UserConstructionScript`)