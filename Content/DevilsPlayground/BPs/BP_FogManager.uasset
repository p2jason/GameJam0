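; Fog manager that, every Tick, encodes villager and light positions into render targets as data for holes in the fog.
; Each BP_Pleb is drawn as one pixel at its array index in RTVillagerFogHoles, with world position in RGB and a fixed radius in alpha.
; BP_Light actors follow for RTLightFogHoles, with alpha as sphere radius scaled by current intensity.
; The light pass reuses the first canvas reference and has no clear or end-draw call.
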(event `self.ReceiveTick`
  (params (DeltaSeconds :type "Float (single-precision)"))
  (bind _rt_villagerfogholes (`self.RT_VillagerFogHoles`))
  (`KismetRenderingLibrary.ClearRenderTarget2D` _rt_villagerfogholes)
  (bind (_canvas _size _context) (`KismetRenderingLibrary.BeginDrawCanvasToRenderTarget` _rt_villagerfogholes))
  (bind _outactors (`GameplayStatics.GetAllActorsOfClass` "/Game/DevilsPlayground/BPs/Characters/BP_Pleb.BP_Pleb_C"))
  (for (_array_element _array_index) _outactors
    (`Canvas.K2_DrawTexture` _canvas null (`KismetMathLibrary.MakeVector2D` (`KismetMathLibrary.Conv_IntToDouble` _array_index)) (1.0 1.0) (0.0 0.0) (1.0 1.0) (`KismetMathLibrary.MakeColor` (.x (`self.K2_GetActorLocation` _array_element)) (.y (`self.K2_GetActorLocation` _array_element)) (.z (`self.K2_GetActorLocation` _array_element)) 1000.0) "BLEND_Opaque" 0.0 (0.5 0.5)))
  (`KismetRenderingLibrary.EndDrawCanvasToRenderTarget` _context)
  (`KismetRenderingLibrary.BeginDrawCanvasToRenderTarget` (`self.RT_LightFogHoles`))
  (bind _outactors_2 (`GameplayStatics.GetAllActorsOfClass` "/Game/DevilsPlayground/Assets/Blockout/BP_Light.BP_Light_C"))
  (for (_array_element_2 _array_index_2) _outactors_2
    (`Canvas.K2_DrawTexture` _canvas null (`KismetMathLibrary.MakeVector2D` (`KismetMathLibrary.Conv_IntToDouble` _array_index_2)) (1.0 1.0) (0.0 0.0) (1.0 1.0) (`KismetMathLibrary.MakeColor` (.x (`self.K2_GetActorLocation` _array_element_2)) (.y (`self.K2_GetActorLocation` _array_element_2)) (.z (`self.K2_GetActorLocation` _array_element_2)) (* (`SphereComponent.GetUnscaledSphereRadius` (`/Game/DevilsPlayground/Assets/Blockout/BP_Light.Sphere` _array_element_2)) (/ (`/Game/DevilsPlayground/Assets/Blockout/BP_Light.CurrentIntensity` _array_element_2) (`/Game/DevilsPlayground/Assets/Blockout/BP_Light.MaxIntensity` _array_element_2)))) "BLEND_Opaque" 0.0 (0.5 0.5))))

(fn `UserConstructionScript`)