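; AI controller for the priest, which starts the BB_Priest blackboard and BT_Priest behavior tree on possession.
; Every tick it writes the player's pawn as TargetWithDevil and a fixed SuspicionRadius to the blackboard, raising a script error unless exactly one BP_PlayerController exists.
; It also runs a per-tick sphere overlap for player actors within ViewDistance, but the loop over the results is empty.
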(event `self.ReceiveBeginPlay`)

(event `self.ReceivePossess`
  (params (PossessedPawn :type "Pawn Object Reference"))
  (bind _blackboardcomponent (`self.UseBlackboard` "/Game/DevilsPlayground/AI/BB_Priest.BB_Priest"))
  (set `self.Blackboard Component` _blackboardcomponent)
  (`self.RunBehaviorTree` "/Game/DevilsPlayground/AI/BT_Priest.BT_Priest"))

(event `self.ReceiveTick`
  (params (DeltaSeconds :type "Float (single-precision)"))
  (bind _blackboard_component (`self.Blackboard Component`))
  (`|ExecutionSequence`
    (:`then_0`
      ; Comment
      (bind _outactors (`GameplayStatics.GetAllActorsOfClass` "/Game/DevilsPlayground/BPs/BP_PlayerController.BP_PlayerController_C"))
      (if (== (`KismetArrayLibrary.Array_Length` _outactors) 1)
        ; Comment
        (`BlackboardComponent.SetValueAsObject` _blackboard_component "TargetWithDevil" (`self.K2_GetPawn` (`|GetArrayItem` _outactors)))
        (`BlackboardComponent.SetValueAsFloat` _blackboard_component "SuspicionRadius" 1000.0)
        (else
          (`KismetSystemLibrary.RaiseScriptError` "Expected only one player controller but found many"))))
    (:`then_1`
      (bind (_outactors_2 _returnvalue) (`KismetSystemLibrary.SphereOverlapActors` (`self.K2_GetActorLocation` (`self.K2_GetPawn`)) (`self.View Distance`) (`|MakeArray` "ObjectTypeQuery2" "ObjectTypeQuery3" :!type "EObjectTypeQuery Enum") (`self.Player Actor Class`)))
      (if _returnvalue
        (for _ _outactors_2
          _)))))

(fn `UserConstructionScript`)